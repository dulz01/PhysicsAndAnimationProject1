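; Phase 2 sector wheel actor that runs a timed rotation and height movement, then hands control to the Phase 1 wheel.
; SetToActive drops it below its start location and enables Tick, which drives the SectorWheelMovement timeline forward, then in reverse.
; Timeline updates yaw it relative to its initial rotation.
; Forward completion sets the timeline height and flags reversal; reverse completion raises it, activates Phase1SectorWheel and deactivates itself.
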(event EventBeginPlay
  (Variables|Default|SetInitial%20Rotation (Transformation|GetActorRotation))
  (Variables|Default|SetInitial%20Location (Transformation|GetActorLocation)))

(event EventTick
  (params (DeltaSeconds :type Float%20%28single-precision%29))
  (bind _returnvalue (Transformation|GetActorLocation))
  (bind _initial_location (Variables|Default|GetInitial%20Location))
  (if (Variables|Default|GetIs%20Active?)
    (if (Variables|Default|GetRevert%20Rotation?)
      (bind (_direction _new_angle _new_height) (Timeline|Sector%20Wheel%20Movement Reverse)
        (:Update
          (Transformation|SetActorRotation (Math|Rotator|CombineRotators (Math|Rotator|MakeRotator 0.0 0.0 _new_angle) (Variables|Default|GetInitial%20Rotation))))
        (:Finished
          (if (Variables|Default|GetRevert%20Rotation?)
            (Transformation|SetActorLocation (Math|Vector|MakeVector (.x _returnvalue) (.y _returnvalue) (+ (.z _returnvalue) 1e+02)) false false)
            (if (Variables|Default|GetIs%20Active?)
              (Default|SettoActive (Variables|Default|GetPhase1SectorWheel))
              (Variables|Default|SetIs%20Active? false))
            (else
              (Transformation|SetActorLocation (Math|Vector|MakeVector (.x _initial_location) (.y _initial_location) (+ _new_height (.z _initial_location))) false false)
              (Variables|Default|SetRevert%20Rotation? true)))))
      (else
        (Timeline|Sector%20Wheel%20Movement Play)))))

(fn ConstructionScript)

(fn SettoActive
  (Transformation|SetActorLocation (- (Variables|Default|GetInitial%20Location) "0, 0,200.000000") false false)
  (Variables|Default|SetIs%20Active? true))